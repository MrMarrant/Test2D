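; BP_Shop is a shop actor that shows a multi-line dialog box with speaker name, text and flipbook portrait.
; Lines come from the DataBoxDialog table, read sequentially by using the index as the row name.
; OpenBoxDialog and NextDialog have no callers here, so they are driven externally.
; Passing the last row or leaving the sphere closes the widget, resets the index and clears BP_Player's dialog state.
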(event `self.ReceiveBeginPlay`
  (`self.GetSizeDataDialog`))

(event `/Game/BluePrints/Interface/BPI_BoxDialog.GetSizeDataDialog`
  ;[1 1 1] Get Size Data Dialog
  (bind _outrownames (`DataTableFunctionLibrary.GetDataTableRowNames` (`self.DataBoxDialog`)))
  (set `self.SizeDialog` (- (`KismetArrayLibrary.Array_Length` _outrownames) 1)))

(event `/Game/BluePrints/Interface/BPI_BoxDialog.OpenBoxDialog`
  ;[1 1 1] Create Box Dialog
  (bind _returnvalue (`|CreateWidget` "/Game/BluePrints/UI/WP_BoxDialog.WP_BoxDialog_C" (`GameplayStatics.GetPlayerController` 0)))
  (bind _output_get (set `self.BoxDialog` _returnvalue))
  (`self.SetRowDialog` "0")
  (`UserWidget.AddToViewport` _output_get 0))

(event `/Game/BluePrints/Interface/BPI_BoxDialog.NextDialog`
  ;[1 1 1] NextDialog
  (if (< (`self.IndexDialog`) (`self.SizeDialog`))
    (bind _output_get (set `self.IndexDialog` (+ (`self.IndexDialog`) 1)))
    (`self.SetRowDialog` (`KismetStringLibrary.Conv_StringToName` (`KismetStringLibrary.Conv_IntToString` _output_get)))
    (else
      (bind _asbp_player (cast `/Game/BluePrints/BP_Player` (`GameplayStatics.GetPlayerCharacter` 0)))
      (`self.CloseBoxDialog` _asbp_player))))

(event `/Game/BluePrints/Interface/BPI_BoxDialog.CloseBoxDialog`
  (params (Player :type "/Game/BluePrints/BP_Player Object Reference"))
  (bind _boxdialog (`self.BoxDialog`))
  ;[1 1 1] Close Box Dialog
  (`/Engine/EditorBlueprintResources/StandardMacros.IsValid` _boxdialog
    (:`Is Valid`
      (`Widget.RemoveFromParent` _boxdialog)
      (set `self.BoxDialog` null)
      (set `self.IndexDialog` 0)
      (set `/Game/BluePrints/BP_Player.IsInDialog` false Player)
      (set `/Game/BluePrints/BP_Player.ActorDialog` null Player))))

(event `self.Sphere.OnComponentEndOverlap`
  (params (OverlappedComponent :type "PrimitiveComponent Object Reference") (OtherActor :type "Actor Object Reference") (OtherComp :type "PrimitiveComponent Object Reference") (OtherBodyIndex :type Integer))
  ;[1 1 1] On End Collision
  (`/Engine/EditorBlueprintResources/StandardMacros.IsValid` (`self.BoxDialog`)
    (:`Is Valid`
      (bind _asbp_player (cast `/Game/BluePrints/BP_Player` OtherActor))
      (`self.CloseBoxDialog` _asbp_player))))

(event `/Game/BluePrints/Interface/BPI_BoxDialog.SetRowDialog`
  (params (Index :type Name))
  (bind _boxdialog (`self.BoxDialog`))
  ;[1 1 1] Set Row Dialog
  (bind _returnvalue (`|GetDataTableRow` (`self.DataBoxDialog`) Index)
    (:`then`
      (bind (_speaker _text _portrait) (break `/Game/Data/DS_BoxDialog` _returnvalue))
      (`/Game/BluePrints/UI/WP_BoxDialog.SetNameSpeaker` _boxdialog _speaker)
      (`/Game/BluePrints/UI/WP_BoxDialog.SetDialogSpeaker` _boxdialog _text)
      (`PaperFlipbookUserWidget.SetFlipbook` (`/Game/BluePrints/UI/WP_BoxDialog.Portrait` _boxdialog) _portrait))))

(fn `UserConstructionScript`)